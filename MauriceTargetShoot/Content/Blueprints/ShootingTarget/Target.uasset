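; Shooting target that jumps to a random point inside its move box on BeginPlay and after each bullet hit.
; On the server, a Bullet_Base hit reports the bullet's owner to FirstPersonGameMode, destroys the bullet, moves the sphere and spawns a BulletPickup.
; Pickups appear at random points using the PickupSpawnBox actors, or spawn with a warning if none are set.
; The construction script sizes the move box from TargetBoundingBoxVector.
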(event `self.ReceiveBeginPlay`
  ;[1 1 1] Get a random starting position
  (`/Engine/EditorBlueprintResources/ActorMacros.Switch Has Authority`
    (:`Authority`
      (`self.Move Sphere to Random Location`))))

(event `self.Sphere.OnComponentHit`
  (params (HitComponent :type "PrimitiveComponent Object Reference") (OtherActor :type "Actor Object Reference") (OtherComp :type "PrimitiveComponent Object Reference") (NormalImpulse :type "Vector Structure") (Hit :type "HitResult Structure (by ref)"))
  (cast `/Game/Blueprints/Bullets/Bullet_Base` OtherActor)
  (`/Engine/EditorBlueprintResources/ActorMacros.Switch Has Authority`
    (:`Authority`
      (bind _asfirst_person_game_mode (cast `/Game/Blueprints/GameMode/FirstPersonGameMode` (`GameplayStatics.GetGameMode`)))
      (`/Game/Blueprints/GameMode/FirstPersonGameMode.HitTarget` _asfirst_person_game_mode (`self.GetOwner` OtherActor))
      (`self.K2_DestroyActor` OtherActor)
      (`self.Move Sphere to Random Location`)
      (`self.SpawnPickup`))))

(fn `Move Sphere to Random Location`
  (`SceneComponent.K2_SetWorldLocation` (`self.Sphere`) (`KismetMathLibrary.RandomPointInBoundingBox` (`SceneComponent.K2_GetComponentLocation` (`self.DefaultSceneRoot`)) (`BoxComponent.BoxExtent` (`self.TargetMoveBox`))) false false))

(fn `SpawnPickup`
  (bind _pickupspawnbox (`self.PickupSpawnBox`))
  (bind _returnvalue (`KismetArrayLibrary.Array_Length` _pickupspawnbox))
  (bind _output (`|GetArrayItem` _pickupspawnbox (`KismetMathLibrary.RandomInteger` (- _returnvalue 1))))
  (if (== _returnvalue 0)
    (`KismetSystemLibrary.PrintString` "No spawnboxes for pickup detected")
    (`|SpawnActorFromClass` "/Game/Blueprints/BulletPickup.BulletPickup_C" (`KismetMathLibrary.MakeTransform` (0.0 0.0 0.0)) "AdjustIfPossibleButAlwaysSpawn" "OverrideRootScale" null null)
    (else
      (`|SpawnActorFromClass` "/Game/Blueprints/BulletPickup.BulletPickup_C" (`KismetMathLibrary.MakeTransform` (`KismetMathLibrary.RandomPointInBoundingBox` (`self.K2_GetActorLocation` _output) (`BoxComponent.BoxExtent` (`/Game/Blueprints/ShootingTarget/PickupBoundigBox.SpawnBox` _output)))) "AdjustIfPossibleButAlwaysSpawn" "OverrideRootScale" null null))))

(fn `UserConstructionScript`
  (`BoxComponent.SetBoxExtent` (`self.TargetMoveBox`) (`self.Target Bounding Box Vector`) false))