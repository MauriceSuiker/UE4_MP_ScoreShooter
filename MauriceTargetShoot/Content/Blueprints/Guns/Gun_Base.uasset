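; Base gun actor owned by a FirstPersonCharacter, handling shooting and magazine reloading in multiplayer.
; Shoot checks loaded ammo, then fires directly with authority or through a server event, where ammo is rechecked against cheating.
; Firing spends a round and spawns a Bullet owned by the player's controller, using the camera's rotation and a rotated muzzle offset.
; Reload follows the same authority routing and tops up the magazine from reserve ammo.
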(event `self.ReceiveBeginPlay`
  ;[1 1 1] Initialize playercontroller so that the bullet spawned knows the owner
  (bind _asfirst_person_character (cast `/Game/Blueprints/FirstPersonCharacter` (`self.GetOwner`)))
  (set `self.PlayerController` (`Pawn.GetController` _asfirst_person_character)))

(event `Shoot`
  (bind _playercontroller (`self.PlayerController`))
  ;[1 1 1] Shoot event called from the character, doesn't really shoot yet
  ;;[1 1 1] First check there are bullets before calling the server
  (if (> (`self.CurrentLoadedAmmo`) 0)
    (`/Engine/EditorBlueprintResources/StandardMacros.IsValid` (`self.PlayerController`)
      (:`Is Valid`
        _)
      (:`Is Not Valid`
        (bind _asfirst_person_character (cast `/Game/Blueprints/FirstPersonCharacter` (`self.GetOwner`)))
        (set `self.PlayerController` (`Pawn.GetController` _asfirst_person_character))))
    (`/Engine/EditorBlueprintResources/ActorMacros.Switch Has Authority`
      (:`Authority`
        (`self.FireBullet` _playercontroller))
      (:`Remote`
        (`self.FireBulletOnServer` _playercontroller)))))

(event `FireBullet`
  (params (Owner :type "Actor Object Reference"))
  ;[1 1 1] The actual shooting part, reducing ammo and spawning a bullet
  ;;[1 1 1] Recheck on the server to prevent cheating
  (if (> (`self.CurrentLoadedAmmo`) 0)
    (set `self.CurrentLoadedAmmo` (- (`self.CurrentLoadedAmmo`) 1))
    (bind _transform (`self.SetBulletTransform`))
    (`|SpawnActorFromClass` (`self.Bullet`) _transform "AdjustIfPossibleButAlwaysSpawn" "OverrideRootScale" Owner null)))

(event `FireBulletOnServer`
  (params (Owner :type "Actor Object Reference"))
  ;[1 1 1] The actual shooting part, reducing ammo and spawning a bullet
  (`self.FireBullet` Owner))

(event `Reload`
  ;[1 1 1] Reloading
  (`/Engine/EditorBlueprintResources/ActorMacros.Switch Has Authority`
    (:`Authority`
      (`self.Reloading`))
    (:`Remote`
      (`self.ReloadOnServer`))))

(event `ReloadOnServer`
  ;[1 1 1] Reloading
  (`self.Reloading`))

(fn `Reloading`
  (locals (Difference :type Integer :default 0))
  (if (not (or (== (`self.CurrentLoadedAmmo`) (`self.MagazineSize`)) (<= (`self.CurrentAmmo`) 0)))
    (bind _output_get (set `local.Difference` (- (`self.MagazineSize`) (`self.CurrentLoadedAmmo`))))
    (if (>= (`self.CurrentAmmo`) _output_get)
      (set `self.CurrentLoadedAmmo` (`self.MagazineSize`))
      (set `self.CurrentAmmo` (- (`self.CurrentAmmo`) (`local.Difference`)))
      (else
        (set `self.CurrentLoadedAmmo` (+ (`self.CurrentLoadedAmmo`) (`self.CurrentAmmo`)))
        (set `self.CurrentAmmo` 0)))))

(fn `SetBulletTransform`
  (returns (Transform :type "Transform Structure"))
  (bind _asfirst_person_character (cast `/Game/Blueprints/FirstPersonCharacter` (`self.GetOwner`)))
  (bind _returnvalue (`SceneComponent.K2_GetComponentRotation` (`/Game/Blueprints/FirstPersonCharacter.FirstPersonCamera` _asfirst_person_character)))
  (return (`KismetMathLibrary.MakeTransform` (+ (`SceneComponent.K2_GetComponentLocation` (`self.BulletSpawnPoint`)) (`KismetMathLibrary.GreaterGreater_VectorRotator` (`self.GunOffset`) _returnvalue)) _returnvalue)))

(fn `UserConstructionScript`)