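; Weapon display actor for the personal room that gives the player a gun on interaction.
; The construction script applies the configurable preview mesh and material to its skeletal mesh, which rotates by a fixed step every tick, independent of frame time.
; Interact casts the interactor to FirstPersonCharacter and calls SpawnWeaponInHand with the configured target gun.
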(event `self.ReceiveTick`
  (params (DeltaSeconds :type "Float (single-precision)"))
  (`SceneComponent.K2_AddLocalRotation` (`self.SkeletalMesh`) (struct :`Yaw` 1.0) false false))

(event `/Game/Blueprints/InteractInterface.Interact`
  (params (Interactor :type "Actor Object Reference"))
  (bind _asfirst_person_character (cast `/Game/Blueprints/FirstPersonCharacter` Interactor))
  (`/Game/Blueprints/FirstPersonCharacter.SpawnWeaponInHand` _asfirst_person_character (`self.TargetGun`)))

(fn `UserConstructionScript`
  (bind _skeletalmesh (`self.SkeletalMesh`))
  (`SkinnedMeshComponent.SetSkinnedAssetAndUpdate` _skeletalmesh (`self.TargetPreview`) true)
  (`PrimitiveComponent.SetMaterial` _skeletalmesh 0 (`self.TargetMaterial`)))