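; DoorTrigger is a personal room door trigger that opens and closes a door only for its owning character.
; On the authority, Box overlap events check that the FirstPersonCharacter matches OwnerDoor, then toggle Closed and call OpenDoor or CloseDoor.
; Both events create a Level Sequence player from DoorSequence on first use, then play it forward to open or in reverse to close.
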(event `OpenDoor`
  (`self.CreatePlayerIfNeeded`)
  (`MovieSceneSequencePlayer.Play` (`self.DoorPlayer`)))

(event `CloseDoor`
  (`self.CreatePlayerIfNeeded`)
  (`MovieSceneSequencePlayer.PlayReverse` (`self.DoorPlayer`)))

(event `self.Box.OnComponentBeginOverlap`
  (params (OverlappedComponent :type "PrimitiveComponent Object Reference") (OtherActor :type "Actor Object Reference") (OtherComp :type "PrimitiveComponent Object Reference") (OtherBodyIndex :type Integer) (bFromSweep :type Boolean) (SweepResult :type "HitResult Structure (by ref)"))
  (bind _asfirst_person_character (cast `/Game/Blueprints/FirstPersonCharacter` OtherActor))
  (`/Engine/EditorBlueprintResources/ActorMacros.Switch Has Authority`
    (:`Authority`
      (if (== _asfirst_person_character (`self.OwnerDoor`))
        (if (`self.Closed`)
          (set `self.Closed` false)
          (`self.OpenDoor`))))))

(event `self.Box.OnComponentEndOverlap`
  (params (OverlappedComponent :type "PrimitiveComponent Object Reference") (OtherActor :type "Actor Object Reference") (OtherComp :type "PrimitiveComponent Object Reference") (OtherBodyIndex :type Integer))
  (bind _asfirst_person_character (cast `/Game/Blueprints/FirstPersonCharacter` OtherActor))
  (`/Engine/EditorBlueprintResources/ActorMacros.Switch Has Authority`
    (:`Authority`
      (if (== _asfirst_person_character (`self.OwnerDoor`))
        (if (not (`self.Closed`))
          (set `self.Closed` true)
          (`self.CloseDoor`))))))

(fn `CreatePlayerIfNeeded`
  (if (not (`KismetSystemLibrary.IsValid` (`self.DoorPlayer`)))
    (bind (_outactor _returnvalue) (`LevelSequencePlayer.CreateLevelSequencePlayer` (`self.DoorSequence`)))
    (set `self.DoorPlayer` _returnvalue))
  (return))

(fn `UserConstructionScript`)