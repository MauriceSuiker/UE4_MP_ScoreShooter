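; SpawnBox is a spawn marker that binds the player who overlaps its sphere to a color-coded personal room door.
; On overlap it records the FirstPersonCharacter as the room trigger's door owner, then branches on its Number, one of four slots.
; Each slot gives the player's capsule a unique collision object channel and colored material, and makes the door block everything except that channel, which only overlaps.
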(event `self.Sphere.OnComponentBeginOverlap`
  (params (OverlappedComponent :type "PrimitiveComponent Object Reference") (OtherActor :type "Actor Object Reference") (OtherComp :type "PrimitiveComponent Object Reference") (OtherBodyIndex :type Integer) (bFromSweep :type Boolean) (SweepResult :type "HitResult Structure (by ref)"))
  (bind _box (`/Game/Blueprints/PersonalRoom/PlayerDoor.Box` (`self.PlayerDoor`)))
  (bind _box_2 (`/Game/Blueprints/PersonalRoom/PlayerDoor.Box` (`self.PlayerDoor`)))
  (bind _box_3 (`/Game/Blueprints/PersonalRoom/PlayerDoor.Box` (`self.PlayerDoor`)))
  (bind _box_4 (`/Game/Blueprints/PersonalRoom/PlayerDoor.Box` (`self.PlayerDoor`)))
  (bind _asfirst_person_character (cast `/Game/Blueprints/FirstPersonCharacter` OtherActor))
  (set `/Game/Blueprints/PersonalRoom/DoorTrigger.OwnerDoor` _asfirst_person_character (`self.DoorTriggerFromRoom`))
  (switch `int` (`self.Number`)
    (:`1`
      ;[1 1 1] Set collision on the door to block other people, change color of the player to easier to remind them which door is theirs
      (`PrimitiveComponent.SetCollisionObjectType` (`Character.CapsuleComponent` _asfirst_person_character) "ECC_GameTraceChannel2")
      (`PrimitiveComponent.SetMaterial` (`/Game/Blueprints/FirstPersonCharacter.Mesh2P` _asfirst_person_character) 0 "/Game/Materials/GreenMat.GreenMat")
      (`PrimitiveComponent.SetCollisionResponseToAllChannels` _box_4 "ECR_Block")
      (`PrimitiveComponent.SetCollisionResponseToChannel` _box_4 "ECC_GameTraceChannel2" "ECR_Overlap"))
    (:`2`
      (`PrimitiveComponent.SetCollisionObjectType` (`Character.CapsuleComponent` _asfirst_person_character) "ECC_GameTraceChannel3")
      (`PrimitiveComponent.SetMaterial` (`/Game/Blueprints/FirstPersonCharacter.Mesh2P` _asfirst_person_character) 0 "/Game/Materials/YellowMat.YellowMat")
      (`PrimitiveComponent.SetCollisionResponseToAllChannels` _box "ECR_Block")
      (`PrimitiveComponent.SetCollisionResponseToChannel` _box "ECC_GameTraceChannel3" "ECR_Overlap"))
    (:`3`
      (`PrimitiveComponent.SetCollisionObjectType` (`Character.CapsuleComponent` _asfirst_person_character) "ECC_GameTraceChannel4")
      (`PrimitiveComponent.SetMaterial` (`/Game/Blueprints/FirstPersonCharacter.Mesh2P` _asfirst_person_character) 0 "/Game/Materials/RedMat.RedMat")
      (`PrimitiveComponent.SetCollisionResponseToAllChannels` _box_3 "ECR_Block")
      (`PrimitiveComponent.SetCollisionResponseToChannel` _box_3 "ECC_GameTraceChannel4" "ECR_Overlap"))
    (:`4`
      (`PrimitiveComponent.SetCollisionObjectType` (`Character.CapsuleComponent` _asfirst_person_character) "ECC_GameTraceChannel5")
      (`PrimitiveComponent.SetMaterial` (`/Game/Blueprints/FirstPersonCharacter.Mesh2P` _asfirst_person_character) 0 "/Game/Materials/BlueMat.BlueMat")
      (`PrimitiveComponent.SetCollisionResponseToAllChannels` _box_2 "ECR_Block")
      (`PrimitiveComponent.SetCollisionResponseToChannel` _box_2 "ECC_GameTraceChannel5" "ECR_Overlap"))))

(fn `UserConstructionScript`)