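; Ammo pickup actor that refills the equipped gun of the FirstPersonCharacter interacting with it.
; Interact adds the gun's PickupAmount, capped at MaxAmmo, then destroys the actor, even if ammo is already full.
; A temporary SpawnSphere, destroyed one second after BeginPlay, plays spawn sound and particles when it overlaps a locally controlled player, limiting feedback to players nearby at spawn.
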(event `self.ReceiveBeginPlay`
  ;[1 1 1] Create a tempory sphere to see if someone is in the 5 meter range
  (`KismetSystemLibrary.K2_SetTimerDelegate` (delegate `DestroySpawnSphere`) 1.0))

(event `DestroySpawnSphere`
  ;[1 1 1] Create a tempory sphere to see if someone is in the 5 meter range
  (`ActorComponent.K2_DestroyComponent` (`self.SpawnSphere`)))

(event `/Game/Blueprints/InteractInterface.Interact`
  (params (Interactor :type "Actor Object Reference"))
  ;[1 1 1] Add ammo if possible and destroy the actor
  (bind _asfirst_person_character (cast `/Game/Blueprints/FirstPersonCharacter` Interactor))
  (bind _equippedgun (`/Game/Blueprints/FirstPersonCharacter.EquippedGun` _asfirst_person_character))
  (bind _currentammo (`/Game/Blueprints/Guns/Gun_Base.CurrentAmmo` _equippedgun))
  (bind _returnvalue (+ (`/Game/Blueprints/Guns/Gun_Base.PickupAmount` _equippedgun) _currentammo))
  (bind _maxammo (`/Game/Blueprints/Guns/Gun_Base.MaxAmmo` _equippedgun))
  (if (<= _returnvalue _maxammo)
    (set `/Game/Blueprints/Guns/Gun_Base.CurrentAmmo` _returnvalue _equippedgun)
    (else
      (set `/Game/Blueprints/Guns/Gun_Base.CurrentAmmo` (+ _currentammo (- _maxammo _currentammo)) _equippedgun)))
  (`self.K2_DestroyActor`))

(event `self.SpawnSphere.OnComponentBeginOverlap`
  (params (OverlappedComponent :type "PrimitiveComponent Object Reference") (OtherActor :type "Actor Object Reference") (OtherComp :type "PrimitiveComponent Object Reference") (OtherBodyIndex :type Integer) (bFromSweep :type Boolean) (SweepResult :type "HitResult Structure (by ref)"))
  (bind _returnvalue (`self.K2_GetActorLocation`))
  ;[1 1 1] Play sound and effect when player is in range during spawning
  (bind _asfirst_person_character (cast `/Game/Blueprints/FirstPersonCharacter` OtherActor))
  (if (`Pawn.IsLocallyControlled` _asfirst_person_character)
    (`GameplayStatics.PlaySoundAtLocation` "/Game/Audio/SpawnPickupSound.SpawnPickupSound" _returnvalue (struct) 1.0 1.0 0.0 null null null)
    (`GameplayStatics.SpawnEmitterAtLocation` "/Game/Particle/SpawnPickupParticle.SpawnPickupParticle" _returnvalue)))

(fn `UserConstructionScript`)